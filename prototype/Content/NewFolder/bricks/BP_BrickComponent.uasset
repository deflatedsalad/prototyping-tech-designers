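; Brick component that snaps a brick's root to a world-space grid when its Initialise event is called.
; Initialise stores the root and its odd-size flags, then rounds the world location up to the horizontal grid in X and Y and to the nearest VerticalIncrements step in Z.
; A half-cell offset is added on each horizontal axis flagged as odd, so such bricks sit between grid lines.
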(event Custom|Initialise
  (params (Brick%20Root :type Scene%20Component%20Object%20Reference) (IsOddX :type Boolean) (IsOddY :type Boolean))
  (Variables|Default|SetBrickRoot Brick%20Root)
  (bind _output_get (Variables|Default|SetIsOddY IsOddY))
  (bind _output_get_2 (Variables|Default|SetisOddX IsOddX))
  (bind _output_get_3 (Variables|Default|SetAdjustmentForOddBricks (Math|Vector|MakeVector (* (Math|Conversions|ToFloat(Boolean) _output_get_2) 2e+01) (* (Math|Conversions|ToFloat(Boolean) _output_get) 2e+01) 0.0)))
  (Transformation|SetWorldLocation (Variables|Default|GetBrickRoot) (+ _output_get_3 (Math|Vector|MakeVector (* (Math|Float|Ceil (.x (/ (Transformation|GetWorldLocation (Variables|Default|GetBrickRoot)) (Math|Vector|MakeVector 4e+01 4e+01 (Variables|Default|Getvertical%20Increments))))) 40) (* (Math|Float|Ceil (.y (/ (Transformation|GetWorldLocation (Variables|Default|GetBrickRoot)) (Math|Vector|MakeVector 4e+01 4e+01 (Variables|Default|Getvertical%20Increments))))) 40) (* (Math|Float|Round (.z (/ (Transformation|GetWorldLocation (Variables|Default|GetBrickRoot)) (Math|Vector|MakeVector 4e+01 4e+01 (Variables|Default|Getvertical%20Increments))))) (Variables|Default|Getvertical%20Increments)))) false false))