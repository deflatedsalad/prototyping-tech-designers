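; BP_Brick is a building-brick actor meant to place box components as stud markers from its stud dimensions.
; IsEven and MoveToLastStud compute the outermost stud offset for odd or even counts.
; Unwired Construction Script logic positions an Arrow there as a cursor, then nested loops attach boxes to the mesh, stepping along Y.
; Nothing currently runs: events are empty and AddStud, duplicating the loop body, is never called.
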(event EventBeginPlay)

(event Collision|EventActorBeginOverlap
  (params (OtherActor :type Actor%20Object%20Reference)))

(fn ConstructionScript)

(fn IsEven
  (params (input :type Float%20%28double-precision%29))
  (bind (_remainder _returnvalue) (Math|Float|Division(WholeandRemainder) input 2.0))
  (return (== _remainder 0.0) _returnvalue))

(fn MovetoLastStud
  (params (input :type Float%20%28double-precision%29))
  (bind (_returnvalue _half_of_studs) (CallFunction|IsEven input))
  (if _returnvalue
    (bind _output_get (Variables|Default|SetTempPos (- (* (Variables|Default|Get1x1%20width) _half_of_studs) 2e+01)))
    (else
      (Variables|Default|SetTempPos (- (* (Variables|Default|Get1x1%20width) (/ (+ input 1.0) 2.0)) 4e+01))))
  (return _output_get))

(fn AddStud
  (params (location :type Vector))
  (Development|PrintString "add brick ran")
  (bind _returnvalue (AddComponent|AddBoxComponent false (Math|Transform|MakeTransform location "0, 0, 0" "0.500000,0.500000,0.500000")))
  (Transformation|AttachComponentToComponent _returnvalue (Variables|Default|GetStaticMesh) "None" "KeepRelative" "KeepRelative" "KeepRelative" true)
  (Utilities|Array|Add (Variables|Default|GetstudPos) _returnvalue)
  (Transformation|AddLocalOffset (Variables|Default|GetArrow) "0.000000,-40.000000,0.000000" false false))