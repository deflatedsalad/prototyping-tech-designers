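; Default third-person player character that moves, jumps, looks and adds the WBP_HUD widget to the viewport when possessed.
; Enhanced Input moves it relative to camera rotation and snaps the mesh yaw to the input direction.
; Look input rotates the spring arm with clamped pitch.
; Grab only runs a debug-drawn capsule trace forward from the camera and prints whether it hit; nothing is picked up.
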(event Input|EnhancedActionEvents|EnhancedInputActionIA_Jump
  (params (ActionValue :type Boolean) (ElapsedSeconds :type Float%20%28double-precision%29) (TriggeredSeconds :type Float%20%28double-precision%29) (InputAction :type Input%20Action%20Object%20Reference :default "/Game/Inputs/IA_Jump.IA_Jump"))
  (Character|Jump))

(event Input|EnhancedActionEvents|EnhancedInputActionIA_Move
  (params (ActionValue :type Vector%202D%20Structure) (ElapsedSeconds :type Float%20%28double-precision%29) (TriggeredSeconds :type Float%20%28double-precision%29) (InputAction :type Input%20Action%20Object%20Reference :default "/Game/Inputs/IA_Move.IA_Move"))
  (bind _returnvalue (Math|Conversions|ToVector(Vector2D) ActionValue))
  (bind _camera (Variables|Default|GetCamera))
  (bind _returnvalue_2 (Transformation|GetWorldRotation _camera))
  (bind _returnvalue_3 (Math|Vector|RotateVector _returnvalue _returnvalue_2))
  (Class|PawnMovementComponent|AddInputVector (Variables|Character|GetCharacterMovement) _returnvalue_3 false)
  (Transformation|SetWorldRotation (Variables|Character|GetMesh) (Math|Rotator|MakeRotator 0.0 0.0 (- (.yaw (Math|Conversions|RotationFromXVector _returnvalue_3)) 9e+01)) false false))

(event Input|EnhancedActionEvents|EnhancedInputActionIA_look
  (params (ActionValue :type Vector%202D%20Structure) (ElapsedSeconds :type Float%20%28double-precision%29) (TriggeredSeconds :type Float%20%28double-precision%29) (InputAction :type Input%20Action%20Object%20Reference :default "/Game/Inputs/IA_look.IA_look"))
  (bind (_x _y) (Math|Vector2D|BreakVector2D ActionValue))
  (bind _springarm (Variables|Default|GetSpringArm))
  (bind _returnvalue (Transformation|GetWorldRotation _springarm))
  (Transformation|SetWorldRotation (Variables|Default|GetSpringArm) (Math|Rotator|MakeRotator 0.0 (Math|Float|Clamp(Float) (+ _y (.pitch _returnvalue)) -35.0 3e+01) (+ _x (.yaw _returnvalue))) false false))

(event Input|EnhancedActionEvents|EnhancedInputActionIA_grab
  (params (ActionValue :type Boolean) (ElapsedSeconds :type Float%20%28double-precision%29) (TriggeredSeconds :type Float%20%28double-precision%29) (InputAction :type Input%20Action%20Object%20Reference :default "/Game/Inputs/IA_grab.IA_grab"))
  (bind _camera (Variables|Default|GetCamera))
  (bind _returnvalue (Transformation|GetWorldLocation _camera))
  (bind _returnvalue_2 (Collision|CapsuleTraceByChannel _returnvalue (+ (* (Math|Vector|GetForwardVector _camera) 1000) _returnvalue) 5e+01 0.0 "TraceTypeQuery3" false 0 "ForDuration"))
  (Development|PrintString (Utilities|String|ToString(Boolean) _returnvalue_2)))

(event EventPossessed
  (params (NewController :type Controller%20Object%20Reference))
  (bind _returnvalue (UserInterface|CreateWidget "/Game/UI/WBP_HUD.WBP_HUD_C"))
  (UserInterface|Viewport|AddtoViewport _returnvalue 0)
  (Development|PrintString "test"))

(event EventUnpossessed
  (params (OldController :type Controller%20Object%20Reference)))

(fn ConstructionScript)